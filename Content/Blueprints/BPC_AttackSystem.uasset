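; Attack component for BP_ThirdPersonCharacter that runs a four-step melee combo of sword attacks and a kick.
; Input starts or buffers attacks, and montage anim notifies continue or reset the combo.
; A looping timer sweeps sphere traces along the sword, while a separate sphere trace covers stab and kick.
; Hits on "Damageable" actors apply damage, camera shake, sound and blood, with the kick montage name selecting unarmed sound without blood.
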(event Custom|Sword%20Attack
  ;[0.05127 0.05127 0.05127] Combo System, the combo continue and stop combo attack sections(below) are all used in the anim notify blue print components and then called by the animation montages. The animation monatges are located in the characters/pirate/animations/attacks folder
  ;;[0.05127 0.05127 0.05127] Sword Attack, is attacking is used for controlling the first hit and save attack is used for controlling the combo continue(below this)
  (if (Variables|Default|GetIs%20Attacking)
    (Variables|Default|SetSave%20Attack true)
    (else
      (Variables|Default|SetIs%20Attacking true)
      (switch int (Variables|Default|GetAttack%20Index)
        (:0
          (CallFunction|Attack1))
        (:1
          (CallFunction|Attack2))
        (:2
          (CallFunction|Attack3))
        (:3
          (CallFunction|Attack4))))))

(event Custom|Sword%20Attack%20Combo
  ;[0.05127 0.05127 0.05127] Combo System, the combo continue and stop combo attack sections(below) are all used in the anim notify blue print components and then called by the animation montages. The animation monatges are located in the characters/pirate/animations/attacks folder
  ;;[0.05127 0.05127 0.05127] Combo Continue, called automatically from the anim notify which is called in the animation monatages. The hit button only serves to set save attack to true so that this will work.
  (if (Variables|Default|GetSave%20Attack)
    (Variables|Default|SetSave%20Attack false)
    (switch int (Variables|Default|GetAttack%20Index)
      (:0
        (CallFunction|Attack1))
      (:1
        (CallFunction|Attack2))
      (:2
        (CallFunction|Attack3))
      (:3
        (CallFunction|Attack4)))
    (else
      (CallFunction|StopCombo))))

(event Custom|Attack%201
  ;[0.05127 0.05127 0.05127] Combo System, the combo continue and stop combo attack sections(below) are all used in the anim notify blue print components and then called by the animation montages. The animation monatges are located in the characters/pirate/animations/attacks folder
  ;;[0.05127 0.05127 0.05127] Attack 1
  (Utilities|FlowControl|DoOnce false :!label _label
    (:Completed
      (Utilities|FlowControl|Delay 0.1)
      (Animation|Montage|PlayMontage (Variables|Default|GetCharacter%20Mesh) "/Game/Characters/Pirate/Animations/Attacks/Sword/Attack1_Montage.Attack1_Montage"
        (:then
          (Variables|Default|SetAttack%20Index 1)
          (goto _label Reset))))))

(event Custom|Play%20Sword%20Hit%20Sounds
  ;[0.05127 0.05127 0.05127] Sounds to play when the enemy gets hit with a sword barring the kick as the kick and sword use similar hurt boxes. I put the blood fx here because it excludes the kick animation
  (bind _newparam (CallFunction|UnarmedAttack))
  (if (not _newparam)
    (Audio|PlaySoundatLocation "/Game/Audio/Sword/MS_SwordHits.MS_SwordHits" (Transformation|GetActorLocation (Components|GetOwner)) "0, 0, 0" 0.7 1.0 0.0 "/Game/Audio/SA_Pirate.SA_Pirate" 0 0 0)
    (else
      (CallFunction|PlayUnarmedHitSound))))

(event Custom|Play%20Unarmed%20Hit%20Sound
  ;[0.05127 0.05127 0.05127] This is for playing unarmed hit sounds
  (Audio|PlaySoundatLocation "/Game/Audio/Grunts_Hits/MS_UnarmedHits.MS_UnarmedHits" (Transformation|GetActorLocation (Components|GetOwner)) "0, 0, 0" 1.0 1.0 0.0 0 0 0 0))

(event Custom|Stop%20Combo
  ;[0.05127 0.05127 0.05127] Combo System, the combo continue and stop combo attack sections(below) are all used in the anim notify blue print components and then called by the animation montages. The animation monatges are located in the characters/pirate/animations/attacks folder
  ;;[0.05127 0.05127 0.05127] Stop Combo/Attack, resets is attacking and the attack index so that we can start from the first attack again this is called from anim notify in the montages
  (Variables|Default|SetIs%20Attacking false)
  (Variables|Default|SetAttack%20Index 0))

(event Custom|Attack%204
  ;[0.05127 0.05127 0.05127] Combo System, the combo continue and stop combo attack sections(below) are all used in the anim notify blue print components and then called by the animation montages. The animation monatges are located in the characters/pirate/animations/attacks folder
  ;;[0.05127 0.05127 0.05127] Attack 4 this is actually actually the attack 3 montage, but I wanted the kick to be before this one and so the kick became 3 and this one is 4.
  (Utilities|FlowControl|DoOnce false :!label _label
    (:Completed
      (Utilities|FlowControl|Delay 0.1)
      (Animation|Montage|PlayMontage (Variables|Default|GetCharacter%20Mesh) "/Game/Characters/Pirate/Animations/Attacks/Sword/Attack3_Montage.Attack3_Montage"
        (:then
          (Variables|Default|SetAttack%20Index 0)
          (goto _label Reset))))))

(event Custom|Sphere%20Trace
  (bind _character_bp (Variables|Default|GetCharacter%20BP))
  (bind _sphere_trace (Variables|/Game/ThirdPerson/Blueprints/BP_ThirdPersonCharacter.BP_ThirdPersonCharacter_C|GetSphere%20Trace _character_bp))
  (bind _returnvalue (Transformation|GetWorldLocation _sphere_trace))
  ;[0.05127 0.05127 0.05127] Sphere Trace (For Stab and Kick). Stab has a very small hit box and because the kick does not use the sword trace, we have to give it a hit box. This sphere trace happens to work out nicely for both.
  (bind (_outhit _returnvalue_2) (Collision|SphereTraceByChannel _returnvalue _returnvalue 25.0 "TraceTypeQuery1" false 0 "None" true "(R=0.918025,G=0.000000,B=1.000000,A=1.000000)"))
  (if _returnvalue_2
    (if (Actor|ActorHasTag (.HitActor (Collision|BreakHitResult _outhit)) "Damageable")
      (CallFunction|CameraShake (.Location (Collision|BreakHitResult _outhit)))
      (Game|Damage|ApplyDamage (.HitActor (Collision|BreakHitResult _outhit)) 1e+01 0 0)
      (bind _newparam (CallFunction|UnarmedAttack))
      (if (not _newparam)
        (Effects|SpawnEmitteratLocation "/Game/FX/Particles/Blood/P_Blood_Splat_Cone.P_Blood_Splat_Cone" (.Location (Collision|BreakHitResult _outhit)) (Math|Rotator|MakeRotfromXY (.Normal (Collision|BreakHitResult _outhit)) (.Normal (Collision|BreakHitResult _outhit))) "0.400000,0.400000,0.400000" true "AutoRelease")))))

(event Custom|Start%20Sword%20Trace
  ;[0.05127 0.05127 0.05127] Sword Trace/ we create a sphere trace around the sword, when it hits, we get the actor it hit and then, if it has a damageable tag, apply damage to the target and cause a camera shake.
  (bind _returnvalue (Utilities|Time|SetTimerbyEvent (delegate Custom|Sword%20Trace%20Loop) 0.01 true))
  (Variables|Default|SetSword%20Trace%20Timer _returnvalue))

(event Custom|Attack%202
  ;[0.05127 0.05127 0.05127] Combo System, the combo continue and stop combo attack sections(below) are all used in the anim notify blue print components and then called by the animation montages. The animation monatges are located in the characters/pirate/animations/attacks folder
  ;;[0.05127 0.05127 0.05127] Attack 2
  (Utilities|FlowControl|DoOnce false :!label _label
    (:Completed
      (Utilities|FlowControl|Delay 0.1)
      (Animation|Montage|PlayMontage (Variables|Default|GetCharacter%20Mesh) "/Game/Characters/Pirate/Animations/Attacks/Sword/Attack2_Montage.Attack2_Montage"
        (:then
          (Variables|Default|SetAttack%20Index 2)
          (goto _label Reset))))))

(event Custom|Sword%20Trace%20Loop
  ;[0.05127 0.05127 0.05127] Sword Trace/ we create a sphere trace around the sword, when it hits, we get the actor it hit and then, if it has a damageable tag, apply damage to the target and cause a camera shake.
  (bind (_outhit _returnvalue) (Collision|SphereTraceByChannel (Transformation|GetWorldLocation (Variables|/Game/ThirdPerson/Blueprints/BP_ThirdPersonCharacter.BP_ThirdPersonCharacter_C|GetSword%20Top%20Point (Variables|Default|GetCharacter%20BP))) (Transformation|GetWorldLocation (Variables|/Game/ThirdPerson/Blueprints/BP_ThirdPersonCharacter.BP_ThirdPersonCharacter_C|GetSword%20Bottom%20Point (Variables|Default|GetCharacter%20BP))) 16.0 "TraceTypeQuery1" false 0 "None" true "(R=1.000000,G=0.000000,B=0.000000,A=1.000000)" "(R=0.000000,G=1.000000,B=0.000000,A=1.000000)" 0.1))
  (if _returnvalue
    (if (Actor|ActorHasTag (.HitActor (Collision|BreakHitResult _outhit)) "Damageable")
      (Utilities|FlowControl|DoOnce false :!label _label
        (:Completed
          (Game|Damage|ApplyDamage (.HitActor (Collision|BreakHitResult _outhit)) 1e+01 0 0)
          (CallFunction|CameraShake (.Location (Collision|BreakHitResult _outhit)))
          (Effects|SpawnEmitteratLocation "/Game/FX/Particles/Blood/P_Blood_Splat_Cone.P_Blood_Splat_Cone" (.Location (Collision|BreakHitResult _outhit)) (Math|Rotator|MakeRotfromXY (.Normal (Collision|BreakHitResult _outhit)) (.Normal (Collision|BreakHitResult _outhit))) "0.400000,0.400000,0.400000" true "AutoRelease")
          (Utilities|FlowControl|Delay 0.2)
          (goto _label Reset))))))

(event Custom|Attack%203
  ;[0.05127 0.05127 0.05127] Combo System, the combo continue and stop combo attack sections(below) are all used in the anim notify blue print components and then called by the animation montages. The animation monatges are located in the characters/pirate/animations/attacks folder
  ;;[0.05127 0.05127 0.05127] Attack 3/Kick
  (Utilities|FlowControl|DoOnce false :!label _label
    (:Completed
      (Utilities|FlowControl|Delay 0.05)
      (Animation|Montage|PlayMontage (Variables|Default|GetCharacter%20Mesh) "/Game/Characters/Pirate/Animations/Attacks/PuchesKicks/Kick_Montage.Kick_Montage"
        (:then
          (Variables|Default|SetAttack%20Index 3)
          (goto _label Reset))))))

(event Custom|Stop%20Sword%20Trace
  ;[0.05127 0.05127 0.05127] Sword Trace/ we create a sphere trace around the sword, when it hits, we get the actor it hit and then, if it has a damageable tag, apply damage to the target and cause a camera shake.
  (Utilities|Time|ClearandInvalidateTimerbyHandle (Variables|Default|GetSword%20Trace%20Timer)))

(event Input|EnhancedActionEvents|EnhancedInputActionIA_Attack
  (params (ActionValue :type Boolean) (ElapsedSeconds :type Float%20%28double-precision%29) (TriggeredSeconds :type Float%20%28double-precision%29) (InputAction :type Input%20Action%20Object%20Reference :default "/Game/ThirdPerson/Input/Actions/IA_Attack.IA_Attack"))
  ;[0.05127 0.05127 0.05127] Combo System, the combo continue and stop combo attack sections(below) are all used in the anim notify blue print components and then called by the animation montages. The animation monatges are located in the characters/pirate/animations/attacks folder
  ;;[0.05127 0.05127 0.05127] Attack Input
  (:Started
    (if (Variables|Default|GetCan%20Attack)
      (CallFunction|SwordAttack))))

(event EventBeginPlay
  ;[0.05127 0.05127 0.05127] Get a reference to the third person character and it's mesh
  (bind _asbp_third_person_character (Utilities|Casting|CastToBP_ThirdPersonCharacter (Components|GetOwner)))
  (Variables|Default|SetCharacter%20BP _asbp_third_person_character)
  (Variables|Default|SetCharacter%20Mesh (Variables|/Script/Engine.Character|GetMesh _asbp_third_person_character)))

(fn CameraShake
  (params (Location :type Vector))
  (Camera|PlayWorldCameraShake "/Game/Blueprints/BP_CameraShake.BP_CameraShake_C" Location 2e+01 2e+03)
  (CallFunction|PlaySwordHitSounds))

(fn UnarmedAttack
  (return (Utilities|Enum|Equal(Enum) (Utilities|GetDisplayName (Animation|Montage|GetCurrentActiveMontage (Components|SkeletalMesh|GetAnimInstance (Variables|/Script/Engine.Character|GetMesh (Variables|Default|GetCharacter%20BP))))) "Kick_Montage")))