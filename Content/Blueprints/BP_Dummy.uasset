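; BP_Dummy is an enemy that a crouched player can kill with a stealth rear assassination.
; An overlap collider shows or hides the assassinate prompt for the player character.
; StealthRearAssassination plays the victim montage, removes prompt and collider, and returns a reference location and actor rotation for the attacker's motion warp.
; It also triggers Ragdoll, which sequences delayed sounds before enabling mesh physics.
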(event OnComponentBeginOverlap(AssassinationRadius)
  (params (OverlappedComponent :type Primitive%20Component%20Object%20Reference) (OtherActor :type Actor%20Object%20Reference) (OtherComp :type Primitive%20Component%20Object%20Reference) (OtherBodyIndex :type Integer) (bFromSweep :type Boolean) (SweepResult :type Hit%20Result%20Structure%20%28by%20ref%29))
  ;[0.05127 0.05127 0.05127] If player is in contact with the assasination collider, show the assassinate prompt
  (bind _asbp_third_person_character (Utilities|Casting|CastToBP_ThirdPersonCharacter OtherActor))
  (if (Variables|/Game/ThirdPerson/Blueprints/BP_ThirdPersonCharacter.BP_ThirdPersonCharacter_C|GetCrouched _asbp_third_person_character)
    (Rendering|SetVisibility (Variables|Default|GetAssassinateWidget) true false)))

(event OnComponentEndOverlap(AssassinationRadius)
  (params (OverlappedComponent :type Primitive%20Component%20Object%20Reference) (OtherActor :type Actor%20Object%20Reference) (OtherComp :type Primitive%20Component%20Object%20Reference) (OtherBodyIndex :type Integer))
  ;[0.05127 0.05127 0.05127] If player leaves the assassination collider, hide the assassination prompt
  (Utilities|Casting|CastToBP_ThirdPersonCharacter OtherActor)
  (Rendering|SetVisibility (Variables|Default|GetAssassinateWidget) false false))

(event Custom|Ragdoll
  ;[0.05127 0.05127 0.05127] Turn the enemy into ragdoll after 2.5 seconds of being assassinated. This gets called in the stealth rear assassination function.
  (Utilities|FlowControl|Delay 0.57)
  (Audio|PlaySoundatLocation (Variables|Default|GetMetasound) (Transformation|GetActorLocation) "0, 0, 0" 1.0 1.0 0.0 0 0 0 0)
  (Utilities|FlowControl|Delay 0.4)
  (Audio|PlaySoundatLocation (Variables|Default|GetMetasound) (Transformation|GetActorLocation) "0, 0, 0" 1.0 1.0 0.0 0 0 0 0)
  (Utilities|FlowControl|Delay 0.69)
  (Audio|PlaySoundatLocation "/Game/Audio/Grunts_Hits/SC_EnemyDeathSounds.SC_EnemyDeathSounds" (Transformation|GetActorLocation) "0, 0, 0" 1.0 1.0 0.0 0 0 0 0)
  (Utilities|FlowControl|Delay 0.2)
  (Physics|SetSimulatePhysics (Variables|Character|GetMesh) true))

(event EventBeginPlay)

(event Collision|EventActorBeginOverlap
  (params (OtherActor :type Actor%20Object%20Reference)))

(fn ConstructionScript)

(fn StealthRearAssassination
  ;[0.05127 0.05127 0.05127] This one gives each instance of the enemy a return node that references the location of the assassin reference and rotation of itself. We can use this to tell our motion warp where to go when we assassinate them.
  (Animation|PlayAnimMontage "/Game/Characters/Pirate/Animations/Assassinations/Knife_Assassination_Victim.Knife_Assassination_Victim" 1.0 "None")
  (CallFunction|Ragdoll)
  (Rendering|SetVisibility (Variables|Default|GetAssassinateWidget) false false)
  (Components|DestroyComponent (Variables|Default|GetAssassination%20Radius))
  (return (Transformation|GetWorldLocation (Variables|Default|GetAssassin%20Reference)) (Transformation|GetActorRotation)))