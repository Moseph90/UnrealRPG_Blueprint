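; Player stats component for BP_ThirdPersonCharacter that tracks current and max health and stamina.
; BeginPlay caches the owning character, and each change function writes straight to that character's HUD widget bars and health text, with SetStats refreshing all of them.
; Increases to current values cap at the max, while decreases return true when the value reaches zero or below, without clamping.
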(event Custom|Set%20Stats
  (bind _player_bp (Variables|Default|GetPlayer%20BP))
  (bind _hud_widget (Variables|/Game/ThirdPerson/Blueprints/BP_ThirdPersonCharacter.BP_ThirdPersonCharacter_C|GetHud%20Widget _player_bp))
  (Progress|SetPercent (Variables|/Game/UI/WB_HUD.WB_HUD_C|GetStaminaBar (Variables|/Game/ThirdPerson/Blueprints/BP_ThirdPersonCharacter.BP_ThirdPersonCharacter_C|GetHud%20Widget (Variables|Default|GetPlayer%20BP))) (/ (Variables|Stamina|GetCurrent%20Stamina) (Variables|Stamina|GetMax%20Stamina)))
  (Progress|SetPercent (Variables|/Game/UI/WB_HUD.WB_HUD_C|GetHealthBar _hud_widget) (/ (Variables|Health|GetCurrent%20Health) (Variables|Health|GetMax%20Health)))
  (Rendering|Components|TextRender|SetText (Variables|/Game/UI/WB_HUD.WB_HUD_C|GetHealthText _hud_widget) (Utilities|Text|ToText(Float) (Variables|Health|GetCurrent%20Health) "HalfToEven")))

(event EventBeginPlay
  (bind _asbp_third_person_character (Utilities|Casting|CastToBP_ThirdPersonCharacter (Components|GetOwner))
    (:then
      (Variables|Default|SetPlayer%20BP _asbp_third_person_character))
    (:CastFailed
      (Development|PrintText "Player reference not found in player stats"))))

(event EventTick
  (params (DeltaSeconds :type Float%20%28single-precision%29)))

(fn DecreaseHealth
  (params (Value :type Float%20%28double-precision%29))
  (bind _player_bp (Variables|Default|GetPlayer%20BP))
  (bind _hud_widget (Variables|/Game/ThirdPerson/Blueprints/BP_ThirdPersonCharacter.BP_ThirdPersonCharacter_C|GetHud%20Widget _player_bp))
  ;[0.05127 0.05127 0.05127] This function decreases health by the value and then returns a boolean called Dead if the health is <= 0.
  (Variables|Health|SetCurrent%20Health (- (Variables|Health|GetCurrent%20Health) Value))
  (Progress|SetPercent (Variables|/Game/UI/WB_HUD.WB_HUD_C|GetHealthBar _hud_widget) (/ (Variables|Health|GetCurrent%20Health) (Variables|Health|GetMax%20Health)))
  (Rendering|Components|TextRender|SetText (Variables|/Game/UI/WB_HUD.WB_HUD_C|GetHealthText _hud_widget) (Utilities|Text|ToText(Float) (Variables|Health|GetCurrent%20Health) "HalfToEven"))
  (if (<= (Variables|Health|GetCurrent%20Health) 0.0)
    (return true)
    (else
      (return false))))

(fn IncreaseMaxHealth
  (params (Value :type Float%20%28double-precision%29))
  (bind _player_bp (Variables|Default|GetPlayer%20BP))
  (bind _hud_widget (Variables|/Game/ThirdPerson/Blueprints/BP_ThirdPersonCharacter.BP_ThirdPersonCharacter_C|GetHud%20Widget _player_bp))
  (Variables|Health|SetMax%20Health (+ (Variables|Health|GetMax%20Health) Value))
  (Progress|SetPercent (Variables|/Game/UI/WB_HUD.WB_HUD_C|GetHealthBar _hud_widget) (/ (Variables|Health|GetCurrent%20Health) (Variables|Health|GetMax%20Health)))
  (Rendering|Components|TextRender|SetText (Variables|/Game/UI/WB_HUD.WB_HUD_C|GetHealthText _hud_widget) (Utilities|Text|ToText(Float) (Variables|Health|GetCurrent%20Health) "HalfToEven")))

(fn DecreaseStamina
  (params (Value :type Float%20%28double-precision%29))
  (Variables|Stamina|SetCurrent%20Stamina (- (Variables|Stamina|GetCurrent%20Stamina) Value))
  (Progress|SetPercent (Variables|/Game/UI/WB_HUD.WB_HUD_C|GetStaminaBar (Variables|/Game/ThirdPerson/Blueprints/BP_ThirdPersonCharacter.BP_ThirdPersonCharacter_C|GetHud%20Widget (Variables|Default|GetPlayer%20BP))) (/ (Variables|Stamina|GetCurrent%20Stamina) (Variables|Stamina|GetMax%20Stamina)))
  (if (<= (Variables|Stamina|GetCurrent%20Stamina) 0.0)
    (return true)
    (else
      (return false))))

(fn IncreaseMaxStamina
  (params (Value :type Float%20%28double-precision%29))
  (Variables|Stamina|SetMax%20Stamina (+ (Variables|Stamina|GetMax%20Stamina) Value))
  (Progress|SetPercent (Variables|/Game/UI/WB_HUD.WB_HUD_C|GetStaminaBar (Variables|/Game/ThirdPerson/Blueprints/BP_ThirdPersonCharacter.BP_ThirdPersonCharacter_C|GetHud%20Widget (Variables|Default|GetPlayer%20BP))) (/ (Variables|Stamina|GetCurrent%20Stamina) (Variables|Stamina|GetMax%20Stamina)))
  (Development|PrintText "Tried to update max stamina"))

(fn IncreaseHealth
  (params (Value :type Float%20%28double-precision%29))
  (bind _player_bp (Variables|Default|GetPlayer%20BP))
  (bind _hud_widget (Variables|/Game/ThirdPerson/Blueprints/BP_ThirdPersonCharacter.BP_ThirdPersonCharacter_C|GetHud%20Widget _player_bp))
  (Variables|Health|SetCurrent%20Health (+ (Variables|Health|GetCurrent%20Health) Value))
  (if (> (Variables|Health|GetCurrent%20Health) (Variables|Health|GetMax%20Health))
    (Variables|Health|SetCurrent%20Health (Variables|Health|GetMax%20Health)))
  (Progress|SetPercent (Variables|/Game/UI/WB_HUD.WB_HUD_C|GetHealthBar _hud_widget) (/ (Variables|Health|GetCurrent%20Health) (Variables|Health|GetMax%20Health)))
  (Rendering|Components|TextRender|SetText (Variables|/Game/UI/WB_HUD.WB_HUD_C|GetHealthText _hud_widget) (Utilities|Text|ToText(Float) (Variables|Health|GetCurrent%20Health) "HalfToEven")))

(fn IncreaseStamina
  (params (Value :type Float%20%28double-precision%29))
  (Variables|Stamina|SetCurrent%20Stamina (+ (Variables|Stamina|GetCurrent%20Stamina) Value))
  (if (> (Variables|Stamina|GetCurrent%20Stamina) (Variables|Stamina|GetMax%20Stamina))
    (Variables|Stamina|SetCurrent%20Stamina (Variables|Stamina|GetMax%20Stamina)))
  (Progress|SetPercent (Variables|/Game/UI/WB_HUD.WB_HUD_C|GetStaminaBar (Variables|/Game/ThirdPerson/Blueprints/BP_ThirdPersonCharacter.BP_ThirdPersonCharacter_C|GetHud%20Widget (Variables|Default|GetPlayer%20BP))) (/ (Variables|Stamina|GetCurrent%20Stamina) (Variables|Stamina|GetMax%20Stamina)))
  (Development|PrintText "Tried to increase stamina"))