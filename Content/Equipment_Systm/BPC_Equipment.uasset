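; BPC_Equipment is a component for BP_ThirdPersonCharacter that handles equipment pickup, inventory storage and the equipment menu.
; Interact sphere-traces forward from the follow camera, adds a hit BP_Equipment's item data to the Inventory array and destroys the actor.
; TogglePause opens or closes the WB_Equipment widget, switching game pause, mouse cursor and input mode.
; The F key prints inventory row names for debugging.
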(event Input|EnhancedActionEvents|EnhancedInputActionIA_Interact
  (params (ActionValue :type Boolean) (ElapsedSeconds :type Float%20%28double-precision%29) (TriggeredSeconds :type Float%20%28double-precision%29) (InputAction :type Input%20Action%20Object%20Reference :default "/Game/ThirdPerson/Input/Actions/IA_Interact.IA_Interact"))
  (bind _follow_camera (Variables|Default|GetFollow%20Camera))
  (bind _returnvalue (Transformation|GetWorldLocation _follow_camera))
  ;[0.05127 0.05127 0.05127] Trace objects to pick up
  (bind (_outhit _returnvalue_2) (Collision|SphereTraceForObjects _returnvalue (+ _returnvalue (* (Math|Vector|GetForwardVector (Transformation|GetWorldRotation _follow_camera)) 5e+02)) 1e+02 (Utilities|Array|MakeArray "ObjectTypeQuery2") false 0 "ForDuration"))
  (if _returnvalue_2
    (bind _asbp_equipment (Utilities|Casting|CastToBP_Equipment (.HitActor (Collision|BreakHitResult _outhit)))
      (:then
        (CallFunction|AddEquipment (Variables|/Game/Equipment_Systm/BP_Equipment.BP_Equipment_C|GetItem%20Data _asbp_equipment))
        (Actor|DestroyActor _asbp_equipment))
      (:CastFailed
        (Development|PrintText "Cast to BP_Equipment failed in BPC_Equipment")))))

(event EventBeginPlay
  (bind _asbp_third_person_character (Utilities|Casting|CastToBP_ThirdPersonCharacter (Components|GetOwner))
    (:then
      (Variables|Default|SetFollow%20Camera (Variables|/Game/ThirdPerson/Blueprints/BP_ThirdPersonCharacter.BP_ThirdPersonCharacter_C|GetFollowCamera _asbp_third_person_character))
      (Variables|Default|SetBP_ThirdPerson _asbp_third_person_character))
    (:CastFailed
      (Development|PrintText "Cast to TPC failed in BPC_Equipment"))))

(event Input|ActionEvents|InputActionTogglePause
  (params (Key :type Key%20Structure :default "None"))
  (bind _returnvalue (Game|GetPlayerController 0))
  ;[0.05127 0.05127 0.05127] Equipment panel menu. This will open the menu at the equipment menu by default, from there we will make tabs that can go to different panels
  (:Pressed
    (if (not (Variables|Default|GetMenu%20Open))
      (Variables|Default|SetMenu%20Open true)
      (Game|SetGamePaused true)
      (bind _returnvalue_2 (UserInterface|CreateWidget "/Game/Equipment_Systm/ui/WB_Equipment.WB_Equipment_C"))
      (bind _output_get (Variables|Default|SetEquipment%20Widget _returnvalue_2))
      (UserInterface|Viewport|AddtoViewport _output_get 0)
      (Variables|/Script/Engine.PlayerController|SetbShowMouseCursor _returnvalue true)
      (Input|SetInputModeGameandUI _returnvalue (Variables|Default|GetEquipment%20Widget) "DoNotLock" false false)
      (else
        (Variables|Default|SetMenu%20Open false)
        (bind _equipment_widget (Variables|Default|GetEquipment%20Widget)
          (:then
            (Widget|RemovefromParent _equipment_widget)
            (Game|SetGamePaused false)
            (Variables|Default|SetEquipment%20Widget 0)
            (Variables|/Script/Engine.PlayerController|SetbShowMouseCursor _returnvalue false)
            (Input|SetInputModeGameOnly _returnvalue false))
          (:else))))))

(event Input|KeyboardEvents|F
  (params (Key :type Key%20Structure :default "None"))
  ;[0.05127 0.05127 0.05127] Trace objects to pick up
  (:Pressed
    (for _array_element (Variables|Default|GetInventory)
      (Development|PrintString (Utilities|String|ToString(Name) (.rowname (.item _array_element)))))))

(fn AddEquipment
  (params (Item :type Struct%20Slots%20Structure%20%28by%20ref%29))
  (Utilities|Array|Add (Variables|Default|GetInventory) Item))